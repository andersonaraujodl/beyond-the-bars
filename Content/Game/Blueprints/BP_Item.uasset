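; BP_Item is a configurable world item that shows interaction icons near the player and destroys itself when interacted with.
; Outer and inner collision spheres switch between two icons by proximity.
; The construction script applies mesh, scale, radii, icon location and debug sphere visibility.
; Tick polls the player's IsInteracting and HitActor to trigger delayed destruction, while the Interact event is empty and its inspect-item spawning logic is disconnected.
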(event `self.InnerCollision.OnComponentBeginOverlap`
  (params (OverlappedComponent :type "PrimitiveComponent Object Reference") (OtherActor :type "Actor Object Reference") (OtherComp :type "PrimitiveComponent Object Reference") (OtherBodyIndex :type Integer) (bFromSweep :type Boolean) (SweepResult :type "HitResult Structure (by ref)"))
  (if (== OtherActor (`GameplayStatics.GetPlayerCharacter` 0))
    (`SceneComponent.SetVisibility` (`self.InnerInteractIcon`) true false)
    (`SceneComponent.SetVisibility` (`self.OuterInteractIcon`) false false)))

(event `self.InnerCollision.OnComponentEndOverlap`
  (params (OverlappedComponent :type "PrimitiveComponent Object Reference") (OtherActor :type "Actor Object Reference") (OtherComp :type "PrimitiveComponent Object Reference") (OtherBodyIndex :type Integer))
  (if (== (`GameplayStatics.GetPlayerCharacter` 0) OtherActor)
    (`SceneComponent.SetVisibility` (`self.InnerInteractIcon`) false false)
    (`SceneComponent.SetVisibility` (`self.OuterInteractIcon`) true false)))

(event `self.OuterCollision.OnComponentBeginOverlap`
  (params (OverlappedComponent :type "PrimitiveComponent Object Reference") (OtherActor :type "Actor Object Reference") (OtherComp :type "PrimitiveComponent Object Reference") (OtherBodyIndex :type Integer) (bFromSweep :type Boolean) (SweepResult :type "HitResult Structure (by ref)"))
  (if (== OtherActor (`GameplayStatics.GetPlayerCharacter` 0))
    (`SceneComponent.SetVisibility` (`self.OuterInteractIcon`) true false)))

(event `self.OuterCollision.OnComponentEndOverlap`
  (params (OverlappedComponent :type "PrimitiveComponent Object Reference") (OtherActor :type "Actor Object Reference") (OtherComp :type "PrimitiveComponent Object Reference") (OtherBodyIndex :type Integer))
  (if (== (`GameplayStatics.GetPlayerCharacter` 0) OtherActor)
    (`SceneComponent.SetVisibility` (`self.OuterInteractIcon`) false false)))

(event `self.ReceiveBeginPlay`
  (bind _asnew_player_character (cast `/Game/Game/NewPlayerCharacter` (`GameplayStatics.GetPlayerCharacter` 0)))
  (set `self.CharacterRef` _asnew_player_character))

(event `self.ReceiveTick`
  (params (DeltaSeconds :type "Float (single-precision)"))
  (bind _characterref (`self.CharacterRef`))
  ;[1 1 1] Interact Unused code
  (if (and (`/Game/Game/NewPlayerCharacter.IsInteracting` _characterref) (== (`/Game/Game/NewPlayerCharacter.Hit Actor` _characterref) self))
    (`self.Interacted`)))

(event `Interacted`
  ;[1 1 1] Interact Unused code
  (`KismetSystemLibrary.Delay` 0.1)
  (`self.K2_DestroyActor`))

(event `/Game/Game/Blueprints/InteractInterface.Interact`
  (params (Interacter :type "/Game/Game/NewPlayerCharacter Object Reference")))

(fn `UserConstructionScript`
  (bind _staticmesh (`self.StaticMesh`))
  (`|ExecutionSequence`
    (:`then_0`
      (`SphereComponent.SetSphereRadius` (`self.InnerCollision`) (`self.InnerSphereRadius`) true)
      (`SphereComponent.SetSphereRadius` (`self.OuterCollision`) (`self.OutterSphereRadius`) true)
      (`SceneComponent.K2_SetRelativeLocation` (`self.InnerInteractIcon`) (`self.Icon Location`) false false)
      (`SceneComponent.K2_SetRelativeLocation` (`self.OuterInteractIcon`) (`self.Icon Location`) false false))
    (:`then_1`
      (`StaticMeshComponent.SetStaticMesh` (`self.StaticMesh`) (`self.Item Mesh`))
      (`SceneComponent.K2_SetWorldTransform` _staticmesh (`KismetMathLibrary.MakeTransform` (`SceneComponent.K2_GetComponentLocation` _staticmesh) (`SceneComponent.K2_GetComponentRotation` _staticmesh) (`self.Item Scale`)) false false))
    (:`then_2`
      (if (`self.IsDebugging`)
        (`SceneComponent.SetVisibility` (`self.InnerCollision`) true false)
        (`SceneComponent.SetVisibility` (`self.OuterCollision`) true false)
        (else
          (`SceneComponent.SetVisibility` (`self.InnerCollision`) false false)
          (`SceneComponent.SetVisibility` (`self.OuterCollision`) false false))))))